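; BP_MainCrystal is the map's central crystal, which runs enemy waves and ends the game through a held interaction.
; StartFight spawns a wave from every BP_EnemySpawn in SpawnPoints immediately, then repeats it on a looping timer.
; InteractStart begins a short countdown that InteractStop cancels.
; If the countdown completes, EndGame calls MULTIEndgame, which opens the level named by LevelName.
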(event `StartFight`
  (bind _returnvalue (`KismetSystemLibrary.K2_SetTimerDelegate` (delegate `SpawnWave`) 20.0 true))
  (set `self.FightTimer` _returnvalue)
  (for _array_element (`self.SpawnPoints`) :!label _label
    (bind _asbp_enemy_spawn (cast `/Game/MNANPrototype/Blueprints/MapComponents/BP_EnemySpawn` _array_element))
    (`/Game/MNANPrototype/Blueprints/MapComponents/BP_EnemySpawn.Spawn Enemy` _asbp_enemy_spawn)))

(event `SpawnWave`
  (goto _label))

(event `/Game/MNANPrototype/Blueprints/BPI_Interact.InteractStart`
  (bind _returnvalue (`KismetSystemLibrary.K2_SetTimerDelegate` (delegate `EndGame`) 5.0))
  (set `self.InteractTimer` _returnvalue))

(event `EndGame`
  (`self.MULTI Endgame`))

(event `/Game/MNANPrototype/Blueprints/BPI_Interact.InteractStop`
  (`KismetSystemLibrary.K2_ClearAndInvalidateTimerHandle` (`self.InteractTimer`)))

(event `MULTI Endgame`
  (`GameplayStatics.OpenLevel` (`self.LevelName`)))

(fn `UserConstructionScript`)