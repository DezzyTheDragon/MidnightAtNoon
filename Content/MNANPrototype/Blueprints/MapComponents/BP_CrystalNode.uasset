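; BP_CrystalNode is an interactable map node that a player disables by holding interact for a short, uninterrupted time.
; Starting interaction on an active node sets a timer that clears NodeActive, and stopping interaction cancels that timer.
; The NodeActive RepNotify hides the node's point light and tells its referenced BP_NodeWall to decrement its node count.
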(event `StartNodeDisable`)

(event `/Game/MNANPrototype/Blueprints/BPI_Interact.InteractStart`
  (if (`self.NodeActive`)
    (bind _returnvalue (`KismetSystemLibrary.K2_SetTimerDelegate` (delegate `DisableNode`) 2.5))
    (set `self.DisableTimerHandle` _returnvalue)))

(event `DisableNode`
  (set `self.NodeActive` false))

(event `CancelNodeDisable`)

(event `/Game/MNANPrototype/Blueprints/BPI_Interact.InteractStop`
  (`KismetSystemLibrary.K2_ClearAndInvalidateTimerHandle` (`self.DisableTimerHandle`)))

(fn `OnRep_NodeActive`
  (`SceneComponent.SetVisibility` (`self.PointLight`) false false)
  (bind _asbp_node_wall (cast `/Game/MNANPrototype/Blueprints/MapComponents/BP_NodeWall` (`self.WallReference`)))
  (`/Game/MNANPrototype/Blueprints/MapComponents/BP_NodeWall.DecrementNodeCount` _asbp_node_wall))

(fn `UserConstructionScript`)