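; BP_ExitTrigger is a map exit zone that ends the match once all hunters are standing in it.
; On the authority, its Box overlap events count "Player"-tagged actors in and out and print the tally against the number of BP_Hunter actors.
; When the count reaches that number, it prints a win message, waits briefly, then calls MULTIEndgame to open the level named by LevelName.
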(event `self.Box.OnComponentBeginOverlap`
  (params (OverlappedComponent :type "PrimitiveComponent Object Reference") (OtherActor :type "Actor Object Reference") (OtherComp :type "PrimitiveComponent Object Reference") (OtherBodyIndex :type Integer) (bFromSweep :type Boolean) (SweepResult :type "HitResult Structure (by ref)"))
  (`/Engine/EditorBlueprintResources/ActorMacros.Switch Has Authority`
    (:`Authority`
      (if (`self.ActorHasTag` OtherActor "Player")
        (set `self.CurrentWaiting` (+ (`self.CurrentWaiting`) 1))
        (bind _outactors (`GameplayStatics.GetAllActorsOfClass` "/Game/MNANPrototype/Blueprints/BP_Hunter.BP_Hunter_C"))
        (bind _returnvalue (`KismetArrayLibrary.Array_Length` _outactors))
        (`KismetSystemLibrary.PrintText` (`|FormatText` "There are {total} out of {count} on the exit" _returnvalue (`self.CurrentWaiting`)))
        (if (>= (`self.CurrentWaiting`) _returnvalue)
          (`KismetSystemLibrary.PrintText` "Winner!!")
          (`KismetSystemLibrary.Delay` 0.5)
          (`self.MULTI Endgame`))))))

(event `MULTI Endgame`
  (`GameplayStatics.OpenLevel` (`self.Level Name`)))

(event `self.Box.OnComponentEndOverlap`
  (params (OverlappedComponent :type "PrimitiveComponent Object Reference") (OtherActor :type "Actor Object Reference") (OtherComp :type "PrimitiveComponent Object Reference") (OtherBodyIndex :type Integer))
  (`/Engine/EditorBlueprintResources/ActorMacros.Switch Has Authority`
    (:`Authority`
      (if (`self.ActorHasTag` OtherActor "Player")
        (set `self.CurrentWaiting` (- (`self.CurrentWaiting`) 1))
        (bind _outactors (`GameplayStatics.GetAllActorsOfClass` "/Game/MNANPrototype/Blueprints/BP_Hunter.BP_Hunter_C"))
        (`KismetSystemLibrary.PrintText` (`|FormatText` "There are {total} out of {count} on the exit" (`KismetArrayLibrary.Array_Length` _outactors) (`self.CurrentWaiting`)))))))

(fn `UserConstructionScript`)