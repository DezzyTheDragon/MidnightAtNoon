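; BP_HunterTrap is a placeable hunter trap that catches a single enemy, printing a debug message when play begins.
; On the authority, its sphere overlap sends HazaredEnteredMessage to the AI controller of the first actor tagged "Enemy", then sets EnemyTrapped to block further triggers.
; Nothing resets that flag, and the Controller_Zombie movement enable/disable logic is disconnected, so it never runs.
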(event `self.ReceiveBeginPlay`
  (`KismetSystemLibrary.PrintString` "Trap placed!"))

(event `self.ReceiveActorBeginOverlap`
  (params (OtherActor :type "Actor Object Reference")))

(event `self.Sphere.OnComponentBeginOverlap`
  (params (OverlappedComponent :type "PrimitiveComponent Object Reference") (OtherActor :type "Actor Object Reference") (OtherComp :type "PrimitiveComponent Object Reference") (OtherBodyIndex :type Integer) (bFromSweep :type Boolean) (SweepResult :type "HitResult Structure (by ref)"))
  (`/Engine/EditorBlueprintResources/ActorMacros.Switch Has Authority`
    (:`Authority`
      (if (and (not (`self.EnemyTrapped`)) (`self.ActorHasTag` OtherActor "Enemy"))
        (message `/Game/MNANPrototype/Blueprints/BPI_Enemy.HazaredEntered` (`AIBlueprintHelperLibrary.GetAIController` OtherActor))
        (set `self.EnemyTrapped` true)))))

(event `self.ReceiveDestroyed`)

(fn `UserConstructionScript`)